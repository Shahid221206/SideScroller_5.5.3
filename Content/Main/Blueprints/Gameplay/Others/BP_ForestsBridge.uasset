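; BP_ForestsBridge is a physics-driven plank bridge built procedurally in the construction script.
; It spawns static mesh planks along local Y, using configurable length and gap values.
; A rotated physics constraint links each neighboring pair at a fixed offset, and the first and last planks have simulation disabled to act as anchors.
; The event graph contains no active logic.
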(event EventBeginPlay)

(event Collision|EventActorBeginOverlap
  (params (OtherActor :type Actor%20Object%20Reference)))

(event EventTick
  (params (DeltaSeconds :type Float%20%28single-precision%29)))

(fn ConstructionScript
  (CallFunction|FGenerateBridge)
  (CallFunction|FGenerateConstraint)
  (Physics|SetSimulatePhysics (Utilities|Array|Get(acopy) (Variables|Default|GetPlanks)) false))

(fn FGenerateBridge
  (for _index (range 0 (Variables|Default|GetPlankLength))
    (bind _returnvalue (AddComponent|AddStaticMeshComponent false (Math|Transform|MakeTransform (Math|Vector|MakeVector 0.0 (Math|Conversions|ToFloat(Integer) (* _index (Variables|Default|GetGapBetweenPlank))) 0.0) "0.000000,0.000000,0.000000" "1.000000,1.150000,1.150000")))
    (Utilities|Array|Add (Variables|Default|GetPlanks) _returnvalue)))

(fn FGenerateConstraint
  (bind _planks (Variables|Default|GetPlanks))
  (for _index (range 0 (- (Variables|Default|GetPlankLength) 1))
    (bind _returnvalue (AddComponent|AddPhysicsConstraintComponent false (Math|Transform|MakeTransform (Math|Vector|MakeVector 0.0 (+ (.y (Variables|/Script/Engine.SceneComponent|GetRelativeLocation (Utilities|Array|Get(acopy) (Variables|Default|GetPlanks) _index))) 13.5) 0.0) "0.000000,0.000000,90.000000" "1.000000,1.000000,1.000000")))
    (Class|PhysicsConstraintComponent|SetConstrainedComponents _returnvalue (Utilities|Array|Get(acopy) _planks _index) "None" (Utilities|Array|Get(acopy) _planks (+ _index 1)) "None")))