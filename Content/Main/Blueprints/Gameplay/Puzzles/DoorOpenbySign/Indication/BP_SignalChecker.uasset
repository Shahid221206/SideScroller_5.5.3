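; Sequence-puzzle checker that validates the order of BP_SignalMain activations against a five-step CorrectIndex combination.
; On BeginPlay it registers itself with every signal and hides its indicator meshes.
; MatchSignal reveals indicators and updates the text as matches progress, showing "PuzzleSolved" on completion.
; A wrong input turns the text red and hides indicators, then after a delay calls CollisionSet on activated signals and restarts the count.
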(event Custom|MatchSignal
  (params (CurrentIndexPass :type Byte))
  (bind _self self)
  (bind _signalsactivated (Variables|Default|GetSignalsActivated))
  (bind _textrender (Variables|Default|GetTextRender))
  (bind _textrender_2 (Variables|Default|GetTextRender))
  (bind _returnvalue (Utilities|GetDisplayName _self))
  (bind _returnvalue_2 (Utilities|String|Append "[" _returnvalue "]"))
  (if (== (Utilities|Array|Get(acopy) (Variables|Default|GetCorrectIndex) (Math|Conversions|ToInteger(Byte) (Variables|Default|GetCount))) CurrentIndexPass)
    (Development|PrintString (Utilities|String|Append _returnvalue_2 "Match Found :-" (Utilities|String|ToString(Byte) (Utilities|Array|Get(acopy) (Variables|Default|GetCorrectIndex) (Math|Conversions|ToInteger(Byte) (Variables|Default|GetCount))))) true true "(R=0.000000,G=0.812500,B=0.122802,A=1.000000)")
    (Rendering|Components|TextRender|SetText (Variables|Default|GetTextRender) (Utilities|Text|ToText(String) (Variables|Default|GetCount)))
    (bind _output_get (Variables|Default|SetCount (+ (Variables|Default|GetCount) 1)))
    (Utilities|FlowControl|Sequence
      (:then_0
        (if (== (Variables|Default|GetCount) 5)
          (bind _output_get_2 (Variables|Default|SetValue "PuzzleSolved"))
          (Rendering|Components|TextRender|SetText (Variables|Default|GetTextRender) _output_get_2)))
      (:then_1
        (for (_array_element _array_index) _signalsactivated
          (if (== _array_index _output_get)
            (Rendering|SetVisibility _array_element true false)))))
    (else
      (Development|PrintString (Utilities|String|Append _returnvalue_2 "Wrong Combination") true true "(R=1.000000,G=0.000000,B=0.168929,A=1.000000)" 5.0)
      (Rendering|Components|TextRender|SetText _textrender_2 (Variables|Default|GetValue))
      (Rendering|Components|TextRender|SetTextRenderColor _textrender_2 (Class|KismetMathLibrary|LinearColortoRGBE "(R=1.000000,G=0.092255,B=0.142018,A=1.000000)"))
      (Utilities|FlowControl|Sequence
        (:then_0
          (for _array_element_2 _signalsactivated
            (Utilities|IsValid _array_element_2
              (:Is%20Valid
                (Rendering|SetVisibility _array_element_2 false false)))))
        (:then_1
          (Utilities|FlowControl|Delay 2.0)
          (for _index (range 0 (- (Utilities|Array|Length (Variables|Default|GetSignalsCheckers)) 1))
            (if (Variables|/Game/Main/Blueprints/Gameplay/Puzzles/DoorOpenbySign/Signal/BP_SignalMain.BP_SignalMain_C|GetActivated (Utilities|Array|Get(acopy) (Variables|Default|GetSignalsCheckers) _index))
              (Default|CollisionSet (Utilities|Array|Get(acopy) (Variables|Default|GetSignalsCheckers) _index) false)))
          (Variables|Default|SetCount 0)
          (Rendering|Components|TextRender|SetText _textrender (Variables|Default|GetValue))
          (Rendering|Components|TextRender|SetTextRenderColor _textrender (Class|KismetMathLibrary|LinearColortoRGBE "(R=0.120684,G=0.828125,B=0.086263,A=1.000000)")))))))

(event EventBeginPlay
  (bind _outactors (Actor|GetAllActorsOfClass "/Game/Main/Blueprints/Gameplay/Puzzles/DoorOpenbySign/Signal/BP_SignalMain.BP_SignalMain_C"))
  (for _array_element _outactors
    (Utilities|Array|Add (Variables|Default|GetSignalsCheckers) _array_element)
    (Variables|/Game/Main/Blueprints/Gameplay/Puzzles/DoorOpenbySign/Signal/BP_SignalMain.BP_SignalMain_C|SetBP_SignalChecker _array_element self)
    (for _array_element_2 (Utilities|Array|MakeArray (Variables|Default|GetCone) (Variables|Default|GetCube) (Variables|Default|GetCircle) (Variables|Default|GetDown) (Variables|Default|GetUp))
      (Utilities|Array|Add (Variables|Default|GetSignalsActivated) _array_element_2)
      (Rendering|SetVisibility _array_element_2 false false))))

(fn ConstructionScript
  (bind _staticmesh (Variables|Default|GetStaticMesh))
  (bind _returnvalue (Rendering|Material|CreateDynamicMaterialInstance _staticmesh 0 (Rendering|Material|GetMaterial _staticmesh 0) "None" :!class /Script/Engine.PrimitiveComponent))
  (bind _output_get (Variables|Default|SetI_Materials _returnvalue))
  (Rendering|Material|SetVectorParameterValue _output_get "Color" (Variables|Default|GetColor) :!class /Script/Engine.MaterialInstanceDynamic)
  (Rendering|Material|SetScalarParameterValue _output_get "Glow" (Variables|Default|GetGlowness) :!class /Script/Engine.MaterialInstanceDynamic))