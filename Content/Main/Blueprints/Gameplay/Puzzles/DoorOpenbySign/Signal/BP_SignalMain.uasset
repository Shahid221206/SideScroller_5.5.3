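; BP_SignalMain is a touchable signal for a puzzle, apparently a door opened by signs.
; When the player overlaps it, it passes its SignalNumbers to BPSignalChecker's MatchSignal, then calls CollisionSet to mark itself activated, hide its mesh and disable collision.
; CollisionSet also accepts false to restore the signal.
; The construction script creates a dynamic material instance to apply per-instance color and glow.
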(event OnComponentBeginOverlap(C_Signal)
  (params (OverlappedComponent :type Primitive%20Component%20Object%20Reference) (OtherActor :type Actor%20Object%20Reference) (OtherComp :type Primitive%20Component%20Object%20Reference) (OtherBodyIndex :type Integer) (bFromSweep :type Boolean) (SweepResult :type Hit%20Result%20Structure%20%28by%20ref%29))
  (if (== OtherActor (Game|GetPlayerCharacter 0))
    (Default|MatchSignal (Variables|Default|GetBP_SignalChecker) (Variables|Default|GetSignalNumbers))
    (CallFunction|CollisionSet true)))

(event Custom|CollisionSet
  (params (StopCollision :type Boolean))
  (Variables|Default|SetActivated StopCollision)
  (Collision|SetCollisionEnabled (Variables|Default|GetC_Signal) (select StopCollision "NoCollision" "QueryOnly"))
  (Development|SetHiddeninGame (Variables|Default|GetSM_MainMesh) StopCollision false))

(event EventBeginPlay)

(fn ConstructionScript
  (bind _sm_mainmesh (Variables|Default|GetSM_MainMesh))
  (bind _returnvalue (Rendering|Material|CreateDynamicMaterialInstance _sm_mainmesh 0 (Rendering|Material|GetMaterial _sm_mainmesh 0) "None" :!class /Script/Engine.PrimitiveComponent))
  (bind _output_get (Variables|Default|SetI_Materials _returnvalue))
  (Rendering|Material|SetVectorParameterValue _output_get "Color" (Variables|Default|GetColor) :!class /Script/Engine.MaterialInstanceDynamic)
  (Rendering|Material|SetScalarParameterValue _output_get "Glow" (Variables|Default|GetGlowness) :!class /Script/Engine.MaterialInstanceDynamic))