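; BP_MovableRock is a falling-stone puzzle actor that spawns a row of BP_Stone actors and defines X-axis patrol bounds.
; On BeginPlay it sets left and right limits around its own position, then spawns count-driven stones from SpawnPoint at fixed spacing toward negative X, storing references.
; DetectionLength flips the RightMove flag outside those limits; this file neither calls it nor applies movement.
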(event Custom|PatrollPoint
  (bind _returnvalue (Transformation|GetActorLocation))
  (bind _distancepatrolling (Variables|Default|GetDistancePatrolling))
  (Variables|Default|SetLeftDistancePatrolling (- (.x _returnvalue) _distancepatrolling))
  (Variables|Default|SetRightDistancePatrolling (+ (.x _returnvalue) _distancepatrolling)))

(event Custom|DetectionLength
  (Variables|Default|SetRightMove (select (< (.x (Transformation|GetActorLocation)) (Variables|Default|GetLeftDistancePatrolling)) true (select (> (.x (Transformation|GetActorLocation)) (Variables|Default|GetRightDistancePatrolling)) false (Variables|Default|GetRightMove)))))

(event EventBeginPlay
  (CallFunction|PatrollPoint)
  (Variables|Default|SetSpawnlocation (Transformation|GetWorldLocation (Variables|Default|GetSpawnPoint)))
  (for _index (range 0 (Math|Conversions|ToInteger(Byte) (Variables|Default|GetSpawnCount)))
    (bind _returnvalue (Game|SpawnActorfromClass "/Game/Main/Blueprints/Gameplay/Puzzles/FallingStone/BP_Stone.BP_Stone_C" (Math|Transform|MakeTransform (- (Variables|Default|GetSpawnlocation) (Math|Vector|MakeVector (* _index 4e+02) 0.0 0.0)) "0, 0, 0" "1.000000,1.000000,1.000000") "Undefined" "MultiplyWithRoot" 0 0))
    (Utilities|Array|Add (Variables|Default|GetStoneRef) _returnvalue)))

(fn ConstructionScript)