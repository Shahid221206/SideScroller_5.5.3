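; BP_Object is a rotate-circle puzzle object that raises and lowers its PullObject component between its starting height and a configurable Distance above it.
; Pull starts a looping timer, with Speed as its interval, that steps the component vertically until it reaches either limit, ignoring new pulls while moving.
; PullUpandDown reverses the last direction, and the Start flag triggers an upward pull on BeginPlay.
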(event Custom|Pull
  (params (UP :type Boolean))
  (if (not (Variables|Default|GetisInProcess))
    (Variables|Default|SetisInProcess true)
    (Variables|Default|SetUP UP)
    (bind _returnvalue (Utilities|Time|SetTimerbyEvent (EventDispatchers|CreateEvent :!event Custom|Process) (Variables|Default|GetSpeed) true))
    (Variables|Default|SetTimer _returnvalue)))

(event Custom|Process
  (bind _pullobject (Variables|Default|GetPullObject))
  (bind _returnvalue (Transformation|GetWorldLocation _pullobject))
  (Transformation|SetWorldLocation _pullobject (Math|Vector|MakeVector (.x _returnvalue) (.y _returnvalue) (select (Variables|Default|GetUP) (+ (.z _returnvalue) 4.0) (- (.z _returnvalue) 4.0))) false false)
  (if (Variables|Default|GetUP)
    (if (>= (.z _returnvalue) (Variables|Default|GetUpLimit))
      (Utilities|Time|ClearandInvalidateTimerbyHandle (Variables|Default|GetTimer) :!label _label)
      (Variables|Default|SetisInProcess false))
    (elif (<= (.z _returnvalue) (Variables|Default|GetOriginal))
      (goto _label))))

(event EventBeginPlay
  (bind _pullobject (Variables|Default|GetPullObject))
  (bind _returnvalue (Transformation|GetWorldLocation _pullobject))
  (Variables|Default|SetUpLimit (+ (.z _returnvalue) (Variables|Default|GetDistance)))
  (Variables|Default|SetOriginal (.z _returnvalue))
  (if (Variables|Default|GetStart)
    (CallFunction|Pull true)))

(event EventPullUpandDown
  (CallFunction|Pull (not (Variables|Default|GetUP))))

(fn ConstructionScript)